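; Survival game mode Blueprint that presents wave progress to the player as the survival state changes.
; On BeginPlay it binds to the state-changed delegate and switches on each state to show wave text widgets, with countdowns for waiting and completed waves.
; When a completed wave's count equals the total, it overrides the enemy spawn delay and briefly afterwards shows "Last Wave".
; All-waves-done and player-death states only print debug messages.
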(event Custom|OnSurvialGameModeStateChanged_Event
  (params (CurrentState :type EWarriorSurvialGameModeState%20Enum :default "WaitSpawnNewWave"))
  (switch Utilities|FlowControl|Switch|SwitchonEWarriorSurvialGameModeState CurrentState
    (:WaitSpawnNewWave
      (CallFunction|CreateWaveWidgetwithCountDown "New Wave ComingIn" (Variables|Default|GetSpawnNewWaveWaitTime)))
    (:SpawningNewWave
      (CallFunction|CreateWaveWidgetNotCountDown (Utilities|Text|FormatText "Wave {CurrentWaveCount}" (Variables|Default|GetCurrentWaveCount))))
    (:WaveCompleted
      (CallFunction|CreateWaveWidgetwithCountDown (Utilities|Text|FormatText "Wave {CurrentWaveCount} Completed" (Variables|Default|GetCurrentWaveCount)) (Variables|Default|GetWaveCompletedWaitTime))
      (if (== (Variables|Default|GetCurrentWaveCount) (Variables|Default|GetTotalWavesToSpawn))
        (Variables|Default|SetSpawnEnemiesDelayTime 4.0)
        (Utilities|FlowControl|Delay 0.2)
        (CallFunction|CreateWaveWidgetNotCountDown "Last Wave")))
    (:AllWavesDone
      (Development|PrintString "All wave Done" true true "(R=0.000000,G=1.000000,B=0.130471,A=1.000000)" 1e+01))
    (:PlayerDied
      (Development|PrintString "Player Dead" true true "(R=1.000000,G=0.040784,B=0.000000,A=1.000000)"))))

(event EventBeginPlay
  (EventDispatchers|AssignOnSurvialGameModeStateChanged (delegate Custom|OnSurvialGameModeStateChanged_Event)))

(event EventTick
  (params (DeltaSeconds :type Float%20%28single-precision%29)))

(fn ConstructionScript)

(fn CreateWaveWidgetwithCountDown
  (params (TextContentToDisplay :type Text) (InTotalCountDownTime :type Float%20%28double-precision%29))
  (bind _returnvalue (Game|ConstructObjectfromClass "/Game/Widgets/GameModeWidgets/WBP_WaveTextWithCountDown.WBP_WaveTextWithCountDown_C"))
  (UserInterface|Viewport|AddtoViewport _returnvalue 0)
  (Rendering|Components|TextRender|SetText (Variables|/Game/Widgets/GameModeWidgets/WBP_WaveTextWithCountDown.WBP_WaveTextWithCountDown_C|GetTextBlock_WaveText _returnvalue) TextContentToDisplay)
  (Default|StartCountDown _returnvalue InTotalCountDownTime))

(fn CreateWaveWidgetNotCountDown
  (params (TextContentToDisplay :type Text))
  (bind _returnvalue (Game|ConstructObjectfromClass "/Game/Widgets/GameModeWidgets/WBP_WaveTextNoCountDown.WBP_WaveTextNoCountDown_C"))
  (UserInterface|Viewport|AddtoViewport _returnvalue 0)
  (Rendering|Components|TextRender|SetText (Variables|/Game/Widgets/GameModeWidgets/WBP_WaveTextNoCountDown.WBP_WaveTextNoCountDown_C|GetTextBlock_WaveText _returnvalue) TextContentToDisplay))